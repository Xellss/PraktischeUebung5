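; Game state Blueprint for a dice-style number placement game on a grid three cells wide.
; SetRNDNumber rolls 1 to 6; SetNumber writes it to cells not flagged set, but stores their flag as false.
; GetTotalNumber sums flagged cells, weighting each by a power of ten from index modulo three.
; GetTotalDigits uses a literal zero instead of the total, and Vector2dToIndex's row-major math is unconnected.
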(event EventBeginPlay)

(event EventTick
  (params (DeltaSeconds :type Float%20%28single-precision%29)))

(fn ConstructionScript)

(fn IsSet
  (params (Index :type Vector%202D%20Structure))
  ;[1 1 1] IsSetFunction
  (return (Utilities|Array|Get(acopy) (Variables|Default|GetBoolArray) (Utilities|Vector2dtoIndex Index))))

(fn GetNumber
  (params (Index :type Vector%202D%20Structure))
  ;[1 1 1] GetNumber
  (bind _result (CallFunction|IsSet Index))
  (if _result
    (return (Utilities|Array|Get(acopy) (Variables|Default|GetIntArray) (Utilities|Vector2dtoIndex Index)))
    (else
      (return -1))))

(fn GetCurrentNumber
  (return (Variables|Default|GetCurrentNumber)))

(fn SetNumber
  (params (Index :type Vector%202D%20Structure))
  (bind _result (Utilities|Vector2dtoIndex Index))
  (bind _result_2 (CallFunction|IsSet Index))
  (if _result_2
    (return)
    (else
      (Utilities|Array|SetArrayElem (Variables|Default|GetIntArray) _result (Variables|Default|GetCurrentNumber))
      (Utilities|Array|SetArrayElem (Variables|Default|GetBoolArray) _result false)
      (return))))

(fn SetRNDNumber
  (Variables|Default|SetCurrentNumber (Math|Random|RandomIntegerinRange 1 6))
  (return))

(fn GetTotalDigits
  (params (Digits :type Integer))
  (return (Math|Integer|%(Integer) (/ 0 (Math|Float|Truncate (Math|Float|Power 1e+01 (Math|Conversions|ToFloat(Integer) Digits)))) 10)))

(fn GetTotalNumber
  (for _index (range 0 9)
    ;[1 1 1] For-Loop
    (bind _out (|Continue _index))
    (LocalVariables|Settotal (+ (* (Math|Float|Truncate (Math|Float|Power 1e+01 (Math|Conversions|ToFloat(Integer) (Math|Integer|%(Integer) _out 3)))) (Utilities|Array|Get(acopy) (Variables|Default|GetIntArray) _index)) (LocalVariables|Gettotal))))
  (return (LocalVariables|Gettotal)))